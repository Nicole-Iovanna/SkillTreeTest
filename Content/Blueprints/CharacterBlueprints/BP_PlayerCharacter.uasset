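; BP_PlayerCharacter is the player character Blueprint, using the Gameplay Ability System for dashing and stamina regeneration.
; It grants GA_Dash on BeginPlay and tries to activate it on Left Shift.
; An attribute-change listener feeds HandleStaminaChange, which restarts GE_Stamina_Regen on any decrease by removing effects granting Status.Stamina.Regen and reapplying it.
; Otherwise, it removes those effects once stamina reaches MaxStamina, so regeneration runs only when needed.
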(event `self.ReceiveBeginPlay`
  (`AbilitySystemComponent.K2_GiveAbility` (`self.AbilitySystemComponent`) "/Game/Blueprints/GameplayAbilities/Abilities/GA_Dash.GA_Dash_C" 0 -1)
  (bind (_asynctaskproxy _attribute _newvalue _oldvalue) (`AbilityAsync_WaitAttributeChanged.WaitForAttributeChanged` null (struct :`AttributeName` "Stamina" :`Attribute` "/Script/SkillTreeTest.BaseAttributeSet:Stamina" :`AttributeOwner` "/Script/CoreUObject.Class'/Script/SkillTreeTest.BaseAttributeSet'"))
    (:`Changed`
      (`self.HandleStaminaChange` _newvalue _oldvalue))))

(event `Key|LeftShift`
  (params (Key :type "Key Structure"))
  (:`Pressed`
    (`AbilitySystemComponent.TryActivateAbilityByClass` (`self.AbilitySystemComponent`) "/Game/Blueprints/GameplayAbilities/Abilities/GA_Dash.GA_Dash_C" true)))

(event `HandleStaminaChange`
  (params (NewValue :type "Float (double-precision)") (OldValue :type "Float (double-precision)"))
  (bind _abilitysystemcomponent (`self.AbilitySystemComponent`))
  (bind (_maxstamina_basevalue _maxstamina_currentvalue) (break `GameplayAttributeData` (`BaseAttributeSet.MaxStamina` (`self.BaseAttributeSet`))))
  (if (< NewValue OldValue)
    (`AbilitySystemComponent.RemoveActiveEffectsWithGrantedTags` _abilitysystemcomponent (struct :`GameplayTags` (struct :`(TagName` "Status.Stamina.Regen"))))
    (`AbilitySystemComponent.BP_ApplyGameplayEffectToSelf` :`self` _abilitysystemcomponent :`GameplayEffectClass` "/Game/Blueprints/GameplayAbilities/Effects/GE_Stamina_Regen.GE_Stamina_Regen_C")
    (elif (>= NewValue _maxstamina_currentvalue)
      (`AbilitySystemComponent.RemoveActiveEffectsWithGrantedTags` _abilitysystemcomponent (struct :`GameplayTags` (struct :`(TagName` "Status.Stamina.Regen")))))))

(fn `UserConstructionScript`)